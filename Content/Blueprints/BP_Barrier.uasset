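; BP_Barrier is an actor that acts as the player's defensive barrier, damaged whenever something overlaps it.
; On BeginPlay it caches the BP_GameState, and each overlap during play reduces the game state's BarrierHealth by PointValue and plays a damage sound.
; When health reaches zero it triggers GameOver, destroys the first BP_Player found in the level and destroys itself.
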(event `self.ReceiveBeginPlay`
  (bind _asbp_game_state (cast `/Game/Blueprints/BP_GameState` (`GameplayStatics.GetGameState`)))
  (set `self.Current Game State` _asbp_game_state))

(event `self.ReceiveActorBeginOverlap`
  (params (OtherActor :type "Actor Object Reference"))
  (bind _current_game_state (`self.Current Game State`))
  (if (not (`/Game/Blueprints/BP_GameState.Is Game Over?` _current_game_state))
    (`/Game/Blueprints/BP_GameState.Reduce Barrier Health` _current_game_state (`self.Point Value`))
    (`GameplayStatics.PlaySound2D` "/Game/Assets/damage.damage" 1.0 1.0 0.0 null null false)
    (if (<= (`/Game/Blueprints/BP_GameState.Barrier Health` _current_game_state) 0)
      (`/Game/Blueprints/BP_GameState.Game Over` _current_game_state)
      (bind _outactors (`GameplayStatics.GetAllActorsOfClass` "/Game/Blueprints/BP_Player.BP_Player_C"))
      (`self.K2_DestroyActor` (`|GetArrayItem` _outactors))
      (`self.K2_DestroyActor`))))

(fn `UserConstructionScript`)