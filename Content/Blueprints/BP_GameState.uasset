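; BP_GameState holds the shared game state: score, barrier health and a game-over flag.
; On BeginPlay it creates WBP_MainUI for the first player controller and adds it to the viewport.
; Events add points to the score and subtract from barrier health, with no clamping or zero check.
; A separate GameOver event sets the flag, shows the UI's game-over text and plays a sound.
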(event `self.ReceiveBeginPlay`
  (bind _returnvalue (`|CreateWidget` "/Game/Blueprints/WBP_MainUI.WBP_MainUI_C" (`GameplayStatics.GetPlayerController` 0)))
  (bind _output_get (set `self.Main UI Reference` _returnvalue))
  (`UserWidget.AddToViewport` _output_get 0))

(event `Increase Score`
  (params (`Point Value` :type Integer))
  (set `self.Score` (+ `Point Value` (`self.Score`))))

(event `Reduce Barrier Health`
  (params (`Point Value` :type Integer))
  (set `self.Barrier Health` (- (`self.Barrier Health`) `Point Value`)))

(event `Game Over`
  (set `self.Is Game Over?` true)
  (`/Game/Blueprints/WBP_MainUI.Show Game Over Text` (`self.Main UI Reference`))
  (`GameplayStatics.PlaySound2D` "/Game/Assets/game-over.game-over" 1.0 1.0 0.0 null null))

(fn `UserConstructionScript`)