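; BP_Enemy is an enemy actor that moves steadily downward along world Z at its Speed.
; On overlap, a Player-tagged actor triggers GameOver on BP_GameState, while a Laser-tagged actor adds PointValue to the score.
; Either hit then destroys both actors and plays an explosion sound at a random pitch.
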(event `self.ReceiveBeginPlay`
  (bind _asbp_game_state (cast `/Game/Blueprints/BP_GameState` (`GameplayStatics.GetGameState`)))
  (set `self.Current Game State` _asbp_game_state))

(event `self.ReceiveTick`
  (params (DeltaSeconds :type "Float (single-precision)"))
  (`self.K2_AddActorWorldOffset` (`KismetMathLibrary.MakeVector` 0.0 0.0 (* (* DeltaSeconds (`self.Speed`)) -1.0))))

(event `self.ReceiveActorBeginOverlap`
  (params (OtherActor :type "Actor Object Reference"))
  (bind _current_game_state (`self.Current Game State`))
  (if (`self.ActorHasTag` OtherActor "Player")
    (`/Game/Blueprints/BP_GameState.Game Over` _current_game_state)
    (`self.K2_DestroyActor` OtherActor :!label _label)
    (`self.K2_DestroyActor`)
    (`GameplayStatics.PlaySound2D` "/Game/Assets/explosion.explosion" 1.0 (`KismetMathLibrary.RandomFloatInRange` 0.5 2.0) 0.0 null null)
    (elif (`self.ActorHasTag` OtherActor "Laser")
      (`/Game/Blueprints/BP_GameState.Increase Score` _current_game_state (`self.Point Value`))
      (goto _label))))

(fn `UserConstructionScript`)