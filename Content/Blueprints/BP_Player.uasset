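; BP_Player is a sprite-based player that follows the mouse horizontally and fires lasers.
; Each tick it deprojects the cursor to world space and moves PlayerSprite to that X, holding Y at zero and Z at the height cached on BeginPlay.
; The IA_FireLaser input calls FireLaser, which spawns BP_Laser at the sprite and plays a shot sound with randomized pitch.
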(event `self.ReceiveBeginPlay`
  (`self.Get Vertical Position`))

(event `self.ReceiveTick`
  (params (DeltaSeconds :type "Float (single-precision)"))
  (bind _returnvalue (`self.GetLocalViewingPlayerController`))
  (bind (_locationx _locationy) (`PlayerController.GetMousePosition` _returnvalue))
  (`SceneComponent.K2_SetWorldLocation` (`self.Player_Sprite`) (`KismetMathLibrary.MakeVector` (.x (`PlayerController.DeprojectScreenPositionToWorld` _returnvalue _locationx _locationy)) 0.0 (`self.Start Z Position`)) false false))

(event `Fire Laser`
  (`|SpawnActorFromClass` "/Game/Blueprints/BP_Laser.BP_Laser_C" (`KismetMathLibrary.Conv_VectorToTransform` (`SceneComponent.K2_GetComponentLocation` (`self.Player_Sprite`))) "Undefined" "MultiplyWithRoot" null null)
  (`GameplayStatics.PlaySound2D` "/Game/Assets/shoot.shoot" 1.0 (`KismetMathLibrary.RandomFloatInRange` 0.5 2.0) 0.0 null null false))

(event `EnhancedInput|/Game/Blueprints/IA_FireLaser`
  (params (ActionValue :type Boolean) (ElapsedSeconds :type "Float (double-precision)") (TriggeredSeconds :type "Float (double-precision)") (InputAction :type "InputAction Object Reference" :default "/Game/Blueprints/IA_FireLaser.IA_FireLaser"))
  (:`Triggered`
    (`self.Fire Laser`)))

(fn `Get Vertical Position`
  (bind (_returnvalue_x _returnvalue_y _returnvalue_z) (`KismetMathLibrary.BreakVector` (`SceneComponent.K2_GetComponentLocation` (`self.Player_Sprite`))))
  (set `self.Start Z Position` _returnvalue_z))

(fn `UserConstructionScript`
  (set `self.Player Camera Reference` (`self.Camera`)))