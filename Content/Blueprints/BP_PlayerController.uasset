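; Player controller that sets up Enhanced Input and lets the player restart the level after game over.
; On begin play it adds the default input mapping context and caches the game state as BP_GameState.
; The restart action reopens the current level by name, but only while the game state reports game over.
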(event `self.ReceiveBeginPlay`
  (`EnhancedInputSubsystemInterface.AddMappingContext` (pcsubsystem `EnhancedInputLocalPlayerSubsystem` self) "/Game/Blueprints/IMC_DefaultLayout.IMC_DefaultLayout" 0 (struct))
  (bind _asbp_game_state (cast `/Game/Blueprints/BP_GameState` (`GameplayStatics.GetGameState`)))
  (set `self.Current Game State` _asbp_game_state))

(event `EnhancedInput|/Game/Blueprints/IA_Restart`
  (params (ActionValue :type Boolean) (ElapsedSeconds :type "Float (double-precision)") (TriggeredSeconds :type "Float (double-precision)") (InputAction :type "InputAction Object Reference" :default "/Game/Blueprints/IA_Restart.IA_Restart"))
  (:`Triggered`
    (if (`/Game/Blueprints/BP_GameState.Is Game Over?` (`self.Current Game State`))
      (bind _returnvalue (`GameplayStatics.GetCurrentLevelName` true))
      (`GameplayStatics.OpenLevel` (`KismetStringLibrary.Conv_StringToName` _returnvalue)))))

(fn `UserConstructionScript`)